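; Inventory component that stores item class and amount pairs in a slot array sized from HG_PlayerController, refreshing the matching grid widget slot on changes.
; AddItem fills partial stacks, then empty slots, recursing on overflow and returning any remainder.
; Using an item calls UseItem on an existing or spawned actor, removing one on success.
; It also drops whole stacks as physics pickups at a camera trace, expands slots and opens an examination widget.
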(event `self.ReceiveBeginPlay`
  (`self.Initialize`))

(event `Initialize`
  (bind _ashg_player_controller (cast `/Game/GameBP/HG_PlayerController` (`GameplayStatics.GetPlayerController` 0) :!pure true))
  (`KismetArrayLibrary.Array_Resize` (`self.InventorySlots`) (`/Game/GameBP/HG_PlayerController.InventorySlots` _ashg_player_controller))
  (`KismetSystemLibrary.Delay` 0.2)
  (set `self.W_InventoryMenuRef` (`/Game/GameBP/HG_PlayerController.W_InventoryMenuRef` _ashg_player_controller))
  (bind _asl1_character (cast `/Game/GameBP/Level1/L1_Character` (`GameplayStatics.GetPlayerCharacter` 0)))
  (set `self.Player Ref` _asl1_character)
  (bind _returnvalue (`|CreateWidget` "/Game/UMG/Inventory/W_Examination.W_Examination_C"))
  (set `self.W_ExaminationRef` _returnvalue)
  (set `/Game/GameBP/HG_PlayerController.W_ExaminationRef` (`self.W_ExaminationRef`) _ashg_player_controller)
  (bind _outactors (`GameplayStatics.GetAllActorsOfClass` "/Game/Blueprints/Actors/Inventory/BP_Examination.BP_Examination_C"))
  (set `self.BP_ExaminationRef` (`|GetArrayItem` _outactors))
  (set `/Game/UMG/Inventory/W_Examination.BPC_InventoryRef` self (`self.W_ExaminationRef`)))

(event `CreateExaminationWidget`
  (params (Index :type Integer))
  (bind _w_inventorymenuref (`self.W_InventoryMenuRef`))
  (`/Game/UMG/Inventory/W_Examination.UpdateWidget` (`self.W_ExaminationRef`) Index)
  (`Widget.SetVisibility` _w_inventorymenuref "Collapsed")
  (`/Engine/EditorBlueprintResources/StandardMacros.IsValid` (`/Game/UMG/Inventory/W_InventoryMenu.W_InventoryDropDown` _w_inventorymenuref)
    (:`Is Valid`
      (`/Game/UMG/Inventory/W_InventoryMenu.CloseDropDownMenu` _w_inventorymenuref))
    (:`Is Not Valid`
      _))
  (`UserWidget.AddToViewport` (`self.W_ExaminationRef`) 2)
  (set `/Game/GameBP/HG_PlayerController.isInventoryOpen` false (cast `/Game/GameBP/HG_PlayerController` (`GameplayStatics.GetPlayerController` 0) :!pure true)))

(fn `AddItem`
  (params (Item :type "/Game/Blueprints/Actors/Inventory/BP_Inventory_Master Class Reference") (Amount :type Integer))
  (returns (`Success?` :type Boolean) (Remainder :type Integer))
  (locals (localItem :type "/Game/Blueprints/Actors/Inventory/BP_Inventory_Master Class Reference") (localAmount :type Integer) (localMaxStackAmount :type Integer) (localIndex :type Integer :default 0))
  (bind (_success_ _index) (`self.CheckForEmptySlot`))
  (bind (_success__2 _index_2) (`self.CheckForEmptySlot`))
  (bind _returnvalue (- (`local.localAmount`) 1))
  (bind (_itemname _icon _description _maxstackamount) (break `/Game/Blueprints/Structs/S_ItemData` (defaults `Object` (`local.localItem`))))
  (bind _returnvalue_2 (+ (`.Amount` (`self.GetItemDataAtIndex` (`local.localIndex`))) (`local.localAmount`)))
  (set `local.localItem` Item)
  (set `local.localAmount` Amount)
  (set `local.localMaxStackAmount` _maxstackamount)
  (if (> _maxstackamount 1)
    (bind (_success__3 _index_3) (`self.CheckForFreeSlot` (`local.localItem`)))
    (if _success__3
      (set `local.localIndex` _index_3)
      (if (> _returnvalue_2 (`local.localMaxStackAmount`))
        (set `local.localAmount` (- _returnvalue_2 (`local.localMaxStackAmount`)))
        (`KismetArrayLibrary.Array_Set` (`self.InventorySlots`) (`local.localIndex`) (make `/Game/Blueprints/Structs/S_InventoryItem` (`local.localItem`) (`local.localMaxStackAmount`)))
        (`self.UpdateInventorySlot` (`local.localIndex`))
        (bind (_success__4 _remainder) (`self.AddItem` (`local.localItem`) (`local.localAmount`)))
        (return true _remainder)
        (else
          (`KismetArrayLibrary.Array_Set` (`self.InventorySlots`) (`local.localIndex`) (make `/Game/Blueprints/Structs/S_InventoryItem` (`local.localItem`) _returnvalue_2))
          (`self.UpdateInventorySlot` (`local.localIndex`))
          (return true 0)))
      (elif _success_
        (set `local.localIndex` _index)
        (if (> (`local.localAmount`) (`local.localMaxStackAmount`))
          (`KismetArrayLibrary.Array_Set` (`self.InventorySlots`) (`local.localIndex`) (make `/Game/Blueprints/Structs/S_InventoryItem` (`local.localItem`) (`local.localMaxStackAmount`)))
          (`self.UpdateInventorySlot` (`local.localIndex`))
          (bind (_success__5 _remainder_2) (`self.AddItem` (`local.localItem`) (- (`local.localAmount`) (`local.localMaxStackAmount`))))
          (return true _remainder_2)
          (else
            (`KismetArrayLibrary.Array_Set` (`self.InventorySlots`) (`local.localIndex`) (make `/Game/Blueprints/Structs/S_InventoryItem` (`local.localItem`) (`local.localAmount`)))
            (`self.UpdateInventorySlot` (`local.localIndex`))
            (return true 0)))
        (else
          (return false (`local.localAmount`)))))
    (elif _success__2
      (set `local.localIndex` _index_2)
      (`KismetArrayLibrary.Array_Set` (`self.InventorySlots`) (`local.localIndex`) (make `/Game/Blueprints/Structs/S_InventoryItem` (`local.localItem`) 1))
      (`self.UpdateInventorySlot` (`local.localIndex`))
      (if (> _returnvalue 0)
        (bind (_success__6 _remainder_3) (`self.AddItem` (`local.localItem`) _returnvalue))
        (return true _remainder_3)
        (else
          (return true 0)))
      (else
        (`KismetSystemLibrary.PrintString` "no free slots")
        (return false (`local.localAmount`))))))

(fn `AddMoreSlots`
  (params (Amount :type Integer))
  (bind _w_inventorymenuref (`self.W_InventoryMenuRef`))
  (bind _ashg_player_controller (cast `/Game/GameBP/HG_PlayerController` (`GameplayStatics.GetPlayerController` 0) :!pure true))
  (bind _w_inventorygrid (`/Game/UMG/Inventory/W_InventoryMenu.W_InventoryGrid` _w_inventorymenuref))
  (bind _output_get (set `/Game/GameBP/HG_PlayerController.InventorySlots` (+ (`/Game/GameBP/HG_PlayerController.InventorySlots` _ashg_player_controller) Amount) _ashg_player_controller))
  (`KismetArrayLibrary.Array_Resize` (`self.InventorySlots`) _output_get)
  (`/Game/UMG/Inventory/W_InventoryGrid.AddMoreSlots` _w_inventorygrid Amount)
  (for _array_element (`/Game/UMG/Inventory/W_InventoryGrid.SlotsArray` _w_inventorygrid)
    (`/Game/UMG/Inventory/W_InventorySlot.Initialize` _array_element _w_inventorymenuref)))

(fn `CheckForEmptySlot`
  (returns (`Success?` :type Boolean) (Index :type Integer))
  (locals (localSuccess :type Boolean) (localIndex :type Integer))
  (for (_array_element _array_index) (`self.InventorySlots`)
    (if (`KismetSystemLibrary.IsValidClass` (`.Item_6_B948984743ED1F2E9E9776A32F5850F6` (break `/Game/Blueprints/Structs/S_InventoryItem` _array_element)))
      (set `local.localSuccess` false)
      (else
        (set `local.localSuccess` true)
        (set `local.localIndex` _array_index)
        (break))))
  (return (`local.localSuccess`) (`local.localIndex`)))

(fn `CheckForFreeSlot`
  (params (Item :type "/Game/Blueprints/Actors/Inventory/BP_Inventory_Master Class Reference"))
  (returns (`Success?` :type Boolean) (Index :type Integer))
  (locals (localSuccess :type Boolean) (localIndex :type Integer))
  (for (_array_element _array_index) (`self.InventorySlots`)
    (bind (_item _amount) (break `/Game/Blueprints/Structs/S_InventoryItem` _array_element))
    (if (and (== _item Item) (< _amount (`.MaxStackAmount_8_DEF95D7348E10181B984E69CA2B46CEB` (break `/Game/Blueprints/Structs/S_ItemData` (defaults `Object` Item)))))
      (set `local.localSuccess` true)
      (set `local.localIndex` _array_index)
      (break)
      (else
        (set `local.localSuccess` false))))
  (return (`local.localSuccess`) (`local.localIndex`)))

(fn `DropItem`
  (params (Index :type Integer))
  (locals (localIndex :type Integer) (localAmount :type Integer :default 0) (localClass :type "/Game/Blueprints/Actors/Inventory/BP_Inventory_Master Class Reference"))
  (bind _camera (`/Game/GameBP/Level1/L1_Character.Camera` (`self.Player Ref`)))
  (bind _returnvalue (`SceneComponent.K2_GetComponentLocation` _camera))
  (bind _output_get (set `local.localIndex` Index))
  (bind (_item _amount) (`self.GetItemDataAtIndex` _output_get))
  (set `local.localAmount` _amount)
  (set `local.localClass` _item)
  (if (> (`local.localAmount`) 0)
    (for _ (range (`local.localAmount`))
      (`self.RemoveItem` (`local.localIndex`)))
    (`/Game/UMG/Inventory/W_InventoryMenu.CloseDropDownMenu` (`self.W_InventoryMenuRef`))
    (bind (_outhit _returnvalue_2) (`KismetSystemLibrary.LineTraceSingle` _returnvalue (+ _returnvalue (* (`SceneComponent.GetForwardVector` _camera) 200.0)) "TraceTypeQuery1"))
    (bind (_bblockinghit _binitialoverlap _time _distance _location _impactpoint _normal _impactnormal _physmat _hitactor _hitcomponent _hitbonename _bonename _hititem _elementindex _faceindex _tracestart _traceend) (`GameplayStatics.BreakHitResult` _outhit))
    (bind _returnvalue_3 (`|SpawnActorFromClass` (`.PickupActor_15_4167A9FC448076B2F9EB969D2F784C30` (break `/Game/Blueprints/Structs/S_ItemData` (defaults `Object` (`local.localClass`)))) (`KismetMathLibrary.MakeTransform` (`KismetMathLibrary.SelectVector` _location _traceend _returnvalue_2)) "Undefined" "MultiplyWithRoot" null null))
    (set `/Game/Blueprints/Actors/Inventory/PickupActors/BP_PickupActor_Master.Amount` (`local.localAmount`) _returnvalue_3)
    (`PrimitiveComponent.SetSimulatePhysics` (`/Game/Blueprints/Actors/Inventory/PickupActors/BP_PickupActor_Master.StaticMesh` _returnvalue_3) true)))

(fn `GetItemDataAtIndex`
  (params (Index :type Integer))
  (returns (Item :type "/Game/Blueprints/Actors/Inventory/BP_Inventory_Master Class Reference") (Amount :type Integer))
  (bind (_item _amount) (break `/Game/Blueprints/Structs/S_InventoryItem` (`|GetArrayItem` (`self.InventorySlots`) Index)))
  (return _item _amount))

(fn `RemoveItem`
  (params (Index :type Integer))
  (bind (_item _amount) (`self.GetItemDataAtIndex` Index))
  (if (> _amount 1)
    (`KismetArrayLibrary.Array_Set` (`self.InventorySlots`) Index (make `/Game/Blueprints/Structs/S_InventoryItem` _item (- _amount 1)))
    (else
      (`KismetArrayLibrary.Array_Set` (`self.InventorySlots`) Index (make `/Game/Blueprints/Structs/S_InventoryItem` null))))
  (`self.UpdateInventorySlot` Index))

(fn `UpdateInventorySlot`
  (params (Index :type Integer))
  (`/Game/UMG/Inventory/W_InventorySlot.UpdateSlot` (`|GetArrayItem` (`/Game/UMG/Inventory/W_InventoryGrid.SlotsArray` (`/Game/UMG/Inventory/W_InventoryMenu.W_InventoryGrid` (`/Game/GameBP/HG_PlayerController.W_InventoryMenuRef` (cast `/Game/GameBP/HG_PlayerController` (`GameplayStatics.GetPlayerController` 0) :!pure true)))) Index)))

(fn `UseItem`
  (params (Index :type Integer))
  (locals (localIndex :type Integer))
  (bind _output_get (set `local.localIndex` Index))
  (bind (_item _amount) (`self.GetItemDataAtIndex` _output_get))
  (if (> _amount 0)
    (bind _returnvalue (`GameplayStatics.GetActorOfClass` _item))
    (`/Engine/EditorBlueprintResources/StandardMacros.IsValid` _returnvalue
      (:`Is Valid`
        (`/Game/Blueprints/Actors/Inventory/BP_Inventory_Master.UseItem` _returnvalue)
        (if (`/Game/Blueprints/Actors/Inventory/BP_Inventory_Master.UseItemSuccess` _returnvalue)
          (`self.RemoveItem` (`local.localIndex`) :!label _label)
          (`/Game/UMG/Inventory/W_InventoryMenu.CloseDropDownMenu` (`self.W_InventoryMenuRef`))
          (else
            (`KismetSystemLibrary.PrintString` "use item no successfull"))))
      (:`Is Not Valid`
        (bind _returnvalue_2 (`|SpawnActorFromClass` _item (`KismetMathLibrary.MakeTransform` (0.0 0.0 0.0)) "Undefined" "MultiplyWithRoot" null null))
        (`/Game/Blueprints/Actors/Inventory/BP_Inventory_Master.UseItem` _returnvalue_2)
        (if (`/Game/Blueprints/Actors/Inventory/BP_Inventory_Master.UseItemSuccess` _returnvalue_2)
          (goto _label))))))