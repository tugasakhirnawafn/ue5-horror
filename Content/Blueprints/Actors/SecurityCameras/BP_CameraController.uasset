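; Interactable camera console that lets the player view and cycle through the level's security cameras.
; It gathers all BP_SecurityCamera actors at BeginPlay, and Interact toggles viewing by swapping the view target.
; While viewing, it takes over input from the character, ignores look input and changes main HUD visibility.
; Space cycles cameras with wraparound, while Return or Action restores player view and control and resets the index.
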(event `self.ReceiveBeginPlay`
  (bind _outactors (`GameplayStatics.GetAllActorsOfClass` "/Game/Blueprints/Actors/SecurityCameras/BP_SecurityCamera.BP_SecurityCamera_C"))
  (set `self.SecurityCameras` _outactors))

(event `/Game/Blueprints/Interfaces/BPI_Interaction.Interact`
  (bind _returnvalue (`GameplayStatics.GetPlayerController` 0))
  (if (`self.isViewingCameras`)
    (`self.LeaveCameraController`)
    (else
      (set `self.isViewingCameras` true)
      (`self.DisableInput` (`GameplayStatics.GetPlayerCharacter` 0) _returnvalue)
      (`Controller.SetIgnoreLookInput` _returnvalue true)
      (`Widget.SetVisibility` (`/Game/GameBP/Level1/L1_Character.MainHUDRef` (cast `/Game/GameBP/Level1/L1_Character` (`GameplayStatics.GetPlayerCharacter` 0) :!pure true)) "Visible")
      (`self.EnableInput` (`GameplayStatics.GetPlayerController` 0))
      (`self.ViewThroughCamera`))))

(event `LeaveCameraController`
  (bind _returnvalue (`GameplayStatics.GetPlayerController` 0))
  (set `self.isViewingCameras` false)
  (`self.DisableInput` _returnvalue)
  (`Controller.ResetIgnoreLookInput` _returnvalue)
  (`Widget.SetVisibility` (`/Game/GameBP/Level1/L1_Character.MainHUDRef` (cast `/Game/GameBP/Level1/L1_Character` (`GameplayStatics.GetPlayerCharacter` 0) :!pure true)) "SelfHitTestInvisible")
  (`self.EnableInput` (`GameplayStatics.GetPlayerCharacter` 0) (`GameplayStatics.GetPlayerController` 0))
  (set `self.CurrentCameraIndex` 0)
  (`PlayerController.SetViewTargetWithBlend` (`GameplayStatics.GetPlayerController` 0) (`GameplayStatics.GetPlayerCharacter` 0) 0.0 "VTBlend_Linear" 0.0 false))

(event `Key|SpaceBar`
  (params (Key :type "Key Structure"))
  (bind _returnvalue (+ (`self.CurrentCameraIndex`) 1))
  (:`Pressed`
    (set `self.CurrentCameraIndex` (select `bool` (> _returnvalue (- (`KismetArrayLibrary.Array_Length` (`self.SecurityCameras`)) 1)) :`false` _returnvalue))
    (`self.ViewThroughCamera`)))

(event `InputAction|Return`
  (params (Key :type "Key Structure"))
  (:`Pressed`
    (`self.LeaveCameraController` :!label _label)))

(event `InputAction|Action`
  (params (Key :type "Key Structure"))
  (:`Pressed`
    (goto _label)))

(fn `UserConstructionScript`)

(fn `ViewThroughCamera`
  (`PlayerController.SetViewTargetWithBlend` (`GameplayStatics.GetPlayerController` 0) (`|GetArrayItem` (`self.SecurityCameras`) (`self.CurrentCameraIndex`)) 0.0 "VTBlend_Linear" 0.0 false)
  (return))