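; BP_MoveableObstacle is an obstacle actor that moves along control points and marks its area as an obstacle for navigation.
; The construction script feeds ControlPoints and Duration into its InterpToMovement component.
; On BeginPlay a NavModifier applies NavArea_Obstacle, then the player character is cached as AI_Classic with proximity defaults.
; An unconnected debug chain would print a count for nearby overlapping obstacles, but never runs.
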(event `self.ReceiveBeginPlay`
  (`NavModifierComponent.SetAreaClass` (`self.NavModifier`) "/Script/NavigationSystem.NavArea_Obstacle")
  (bind _asai_classic (cast `/Game/AI/Classic/AI_Classic` (`GameplayStatics.GetPlayerCharacter` 0)))
  (set `self.AIClassicRef` _asai_classic)
  (set `self.ObstacleCount` 0)
  (set `self.MinProximityDistance` 200.0))

(event `self.SM_Hallway_Ceiling_Slat_600.OnComponentBeginOverlap`
  (params (OverlappedComponent :type "PrimitiveComponent Object Reference") (OtherActor :type "Actor Object Reference") (OtherComp :type "PrimitiveComponent Object Reference") (OtherBodyIndex :type Integer) (bFromSweep :type Boolean) (SweepResult :type "HitResult Structure (by ref)")))

(fn `UserConstructionScript`
  (bind _interptomovement (`self.InterpToMovement`))
  (set `InterpToMovementComponent.ControlPoints` (`self.ControlPoints`) _interptomovement)
  (set `InterpToMovementComponent.Duration` (`self.Duration`) _interptomovement))