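; BP_HideActor_Locker is a locker hiding spot, extending a parent hide actor with an animated door.
; Interact swings the door open by timeline, calls the parent Interact, and on alternate uses turns the player's control yaw to match HidingPosition.
; The parent's FinishedMoving dispatcher triggers the door to close, which re-enables interaction.
; The FlipFlop runs before the CanInteract check, so blocked presses still toggle the rotation flag.
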(event `self.ReceiveBeginPlay`
  (`parent.ReceiveBeginPlay`)
  (add `self.FinishedMovingED` (delegate `FinishedMovingED_Event`)))

(event `FinishedMovingED_Event`
  (`KismetSystemLibrary.Delay` 0.2)
  (`self.CloseDoor`))

(event `/Game/Blueprints/Interfaces/BPI_Interaction.Interact`
  (`/Engine/EditorBlueprintResources/StandardMacros.FlipFlop`
    (:`A`
      (set `self.ShouldRotate?` true))
    (:`B`
      (set `self.ShouldRotate?` false)))
  (if (`self.canInteract`)
    (set `self.canInteract` false)
    (bind (_direction _alpha) (`Timeline|OpenLockerDoorTL` :!via `PlayFromStart`)
      (:`Update`
        (`SceneComponent.K2_SetRelativeRotation` (`self.StaticMesh1`) (`KismetMathLibrary.MakeRotator` 0.0 0.0 (`KismetMathLibrary.Lerp` 0.0 90.0 _alpha)) false false))
      (:`Finished`
        (`KismetSystemLibrary.Delay` 0.2)
        (`parent.Interact`)
        (`self.RotatePlayer`)))))

(event `CloseDoor`
  (bind (_direction _alpha) (`Timeline|CloseDoorTL` :!via `PlayFromStart`)
    (:`Update`
      (`SceneComponent.K2_SetRelativeRotation` (`self.StaticMesh1`) (`KismetMathLibrary.MakeRotator` 0.0 0.0 (`KismetMathLibrary.Lerp` 90.0 0.0 _alpha)) false false))
    (:`Finished`
      (set `self.canInteract` true))))

(event `RotatePlayer`
  (bind _returnvalue (`GameplayStatics.GetPlayerCharacter` 0))
  (bind (_returnvalue_roll _returnvalue_pitch _returnvalue_yaw) (`KismetMathLibrary.BreakRotator` (`Pawn.GetControlRotation` _returnvalue)))
  (bind (_returnvalue_roll_2 _returnvalue_pitch_2 _returnvalue_yaw_2) (`KismetMathLibrary.BreakRotator` (`SceneComponent.K2_GetComponentRotation` (`self.HidingPosition`))))
  (if (`self.ShouldRotate?`)
    (bind _output_get (set `self.InitialYAWRotation` _returnvalue_yaw))
    (bind (_direction _alpha) (`Timeline|RotatePlayerTL` :!via `PlayFromStart`)
      (:`Update`
        (`Controller.SetControlRotation` (`Pawn.GetController` _returnvalue) (`KismetMathLibrary.MakeRotator` 0.0 0.0 (`|EaseFunction` "Linear" _alpha _output_get _returnvalue_yaw_2)))))))

(fn `UserConstructionScript`
  (`parent.UserConstructionScript`))