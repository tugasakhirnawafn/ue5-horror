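; A ten-position numbered dial for a lock puzzle, starting on a random digit and turned by two arrow widgets.
; One timeline rolls the mesh a 36-degree step, playing forward or in reverse for direction, while a flag blocks overlapping turns.
; After each step it wraps the rotation within a full circle, derives the digit from the angle and tells the parent lock to recheck.
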(event `self.ReceiveBeginPlay`
  (`/Game/UMG/W_Arrow.Initialize` (cast `/Game/UMG/W_Arrow` (`WidgetComponent.GetUserWidgetObject` (`self.UpArrow`)) :!pure true) self true)
  (`/Game/UMG/W_Arrow.Initialize` (cast `/Game/UMG/W_Arrow` (`WidgetComponent.GetUserWidgetObject` (`self.DownArrow`)) :!pure true) self false)
  (`self.SetRandomNumber`))

(event `FindNumber`
  (bind _output_get (set `self.Number` (`KismetMathLibrary.Abs_Int` (`KismetMathLibrary.FTrunc` (/ (`self.DialRotation`) 36.0)))))
  (`KismetSystemLibrary.PrintString` (`KismetStringLibrary.Conv_IntToString` _output_get)))

(event `RotateDial`
  (bind _dialrotation (`self.DialRotation`))
  (if (`self.canRotate`)
    (set `self.canRotate` false)
    (bind (_direction _alpha) (`Timeline|RotateDialTL` :!via `PlayFromStart` :!label _label)
      (:`Update`
        (bind _returnvalue (+ (`self.DialRotation`) (select `ETimelineDirection` _direction :`Forward` (`KismetMathLibrary.Lerp` 0.0 36.0 _alpha) :`Backward` (`KismetMathLibrary.Lerp` -36.0 0.0 _alpha))))
        (`SceneComponent.K2_SetRelativeRotation` (`self.LockDialMesh`) (`KismetMathLibrary.MakeRotator` _returnvalue) false false))
      (:`Finished`
        (set `self.DialRotation` _returnvalue)
        (if (>= _dialrotation 360.0)
          (set `self.DialRotation` 0.0)
          (`SceneComponent.K2_SetRelativeRotation` :`self` (`self.LockDialMesh`))
          (elif (< _dialrotation 0.0)
            (bind _output_get (set `self.DialRotation` (`KismetMathLibrary.MapRangeClamped` (`self.DialRotation`) 0.0 -360.0 360.0)))
            (`SceneComponent.K2_SetRelativeRotation` (`self.LockDialMesh`) (`KismetMathLibrary.MakeRotator` _output_get) false false)))
        (`self.FindNumber`)
        (`/Game/Blueprints/Actors/BP_Lock.CheckEveryTurn` (`self.BPLockRef`))
        (set `self.canRotate` true)))))

(event `RotateDialBackwards`
  (if (`self.canRotate`)
    (set `self.canRotate` false)
    (goto _label :!via `ReverseFromEnd`)))

(fn `SetRandomNumber`
  (locals (localRotation :type "Float (double-precision)"))
  (set `local.localRotation` (* (`KismetMathLibrary.RandomIntegerInRange` 0 9) 36))
  (`SceneComponent.K2_SetRelativeRotation` (`self.LockDialMesh`) (`KismetMathLibrary.MakeRotator` (`local.localRotation`)) false false)
  (set `self.DialRotation` (`local.localRotation`))
  (`self.FindNumber`))

(fn `UserConstructionScript`)