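; Bandage inventory item that restores player health when used.
; Its UseItem event checks the player's BPCHealth component and, if current health is below maximum, adds AmountOfHealthToAdd.
; It sets UseItemSuccess to report whether the heal was applied, failing when health is already full.
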(event `self.UseItem`
  (bind _bpc_health (`/Game/GameBP/Level1/L1_Character.BPC_Health` (`self.PlayerRef`)))
  (if (< (`/Game/Blueprints/BlueprintComponents/BPC_Health.CurrentHealth` _bpc_health) (`/Game/Blueprints/BlueprintComponents/BPC_Health.MaxHealth` _bpc_health))
    (`/Game/Blueprints/BlueprintComponents/BPC_Health.AddHealth` _bpc_health (`self.AmountOfHealthToAdd`))
    (set `self.UseItemSuccess` true)
    (else
      (set `self.UseItemSuccess` false))))

(fn `UserConstructionScript`
  (`parent.UserConstructionScript`))